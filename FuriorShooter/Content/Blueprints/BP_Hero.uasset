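; BP_Hero is the player-controlled hero, moving with inertia in the X-Z plane using forward and up vectors.
; Horizontal and Vertical axis inputs accumulate acceleration into two velocity variables, which Tick feeds into movement input.
; Tick consumes that input, scales it by delta time, clamps it to MaxVelocity with Y zeroed, and passes it to NiceMove.
; Both velocities then decay by a per-frame deceleration factor that is not scaled by delta time.
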(event EventBeginPlay)

(event Collision|EventActorBeginOverlap
  (params (OtherActor :type Actor%20Object%20Reference)))

(event EventTick
  (params (DeltaSeconds :type Float%20%28single-precision%29))
  (Utilities|FlowControl|Sequence
    (:then_0
      (Pawn|Input|AddMovementInput (Transformation|GetActorForwardVector) (Variables|Default|GetHorizVelocity) false)
      (Pawn|Input|AddMovementInput (Transformation|GetActorUpVector) (Variables|Default|GetVerticalVelocity) false))
    (:then_1
      (bind _returnvalue (Class|Pawn|ConsumeMovementInputVector))
      (bind _normalizedvelocity (CallFunction|NormalizeVelocity (* _returnvalue DeltaSeconds)))
      (Class|Hero|NiceMove _normalizedvelocity))
    (:then_2
      (CallFunction|ApplyDeceleration))))

(event Input|AxisEvents|InputAxisHorizontal
  (params (AxisValue :type Float%20%28single-precision%29))
  ;[1 1 1] Acceleration
  (Variables|Default|SetHorizVelocity (+ (Variables|Default|GetHorizVelocity) (* AxisValue (Variables|Default|GetAcceleration)))))

(event Input|AxisEvents|InputAxisVertical
  (params (AxisValue :type Float%20%28single-precision%29))
  ;[1 1 1] Acceleration
  (Variables|Default|SetVerticalVelocity (+ (Variables|Default|GetVerticalVelocity) (* AxisValue (Variables|Default|GetAcceleration)))))

(fn ConstructionScript)

(fn NormalizeVelocity
  (params (InputVelocity :type Vector))
  (bind _maxvelocity (Variables|Default|GetMaxVelocity))
  (bind _output_get (LocalVariables|SetVelocity (Math|Vector2D|MakeVector2D (.x InputVelocity) (.z InputVelocity))))
  (if (> (Class|KismetMathLibrary|VSize2DSquared _output_get) (Math|Float|Square (Variables|Default|GetMaxVelocity)))
    (return (Math|Vector|MakeVector (* _maxvelocity (.x (Math|Vector2D|Normalize2D (LocalVariables|GetVelocity)))) 0.0 (* _maxvelocity (.y (Math|Vector2D|Normalize2D (LocalVariables|GetVelocity))))))
    (else
      (return (Math|Vector|MakeVector (.x InputVelocity) 0.0 (.z InputVelocity))))))

(fn ApplyDeceleration
  (bind _decelerationfactor (Variables|Default|GetDecelerationFactor))
  (Variables|Default|SetVerticalVelocity (* _decelerationfactor (Variables|Default|GetVerticalVelocity)))
  (Variables|Default|SetHorizVelocity (* _decelerationfactor (Variables|Default|GetHorizVelocity))))